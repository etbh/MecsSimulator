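; PropheteBp is a player-controlled prophet character moved along world axes by input.
; MoveUp and MoveRigt axis inputs feed movement along world X and Y respectively.
; On BeginPlay it spawns a SphereDeCollisionBp at its capsule's transform, scaled up thirtyfold, and passes itself to that sphere as Monprophete.
; Hit, overlap and Tick events are empty.
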(event `InputAxis|MoveRigt`
  (params (AxisValue :type "Float (single-precision)"))
  (`self.AddMovementInput` (0.0 1.0 0.0) AxisValue))

(event `InputAxis|MoveUp`
  (params (AxisValue :type "Float (single-precision)"))
  (`self.AddMovementInput` (1.0 0.0 0.0) AxisValue))

(event `self.ReceiveHit`
  (params (MyComp :type "PrimitiveComponent Object Reference") (Other :type "Actor Object Reference") (OtherComp :type "PrimitiveComponent Object Reference") (bSelfMoved :type Boolean) (HitLocation :type "Vector Structure") (HitNormal :type "Vector Structure") (NormalImpulse :type "Vector Structure") (Hit :type "HitResult Structure (by ref)")))

(event `self.ReceiveBeginPlay`
  (bind _returnvalue (`|SpawnActorFromClass` "/Game/Enterotest/SphereDeCollisionBp.SphereDeCollisionBp_C" (`KismetMathLibrary.MakeTransform` (.location (`SceneComponent.K2_GetComponentToWorld` (`self.CapsuleComponent`))) (.rotation (`SceneComponent.K2_GetComponentToWorld` (`self.CapsuleComponent`))) (30.0 30.0 30.0)) "AlwaysSpawn" "OverrideRootScale"))
  (set `/Game/Enterotest/SphereDeCollisionBp.Monprophete` self _returnvalue))

(event `self.ReceiveActorBeginOverlap`
  (params (OtherActor :type "Actor Object Reference")))

(event `self.ReceiveTick`
  (params (DeltaSeconds :type "Float (single-precision)")))

(fn `UserConstructionScript`)