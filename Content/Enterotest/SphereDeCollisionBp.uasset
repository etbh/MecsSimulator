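; Influence sphere that follows its prophet (Monprophete), converting Neutre Fidele actors and steering those inside it.
; On overlap, a neutral Fidele takes the prophet's faction and color through a dynamic material.
; Each tick, same-faction detections apply go-away (cursor ray-plane intersection), follow-me or a (-1,-1,-1) destination.
; Nested loops apply destinations to every overlapping Fidele regardless of faction; other-faction detections send all to a non-neutral prophet.
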(event `self.ReceiveActorBeginOverlap`
  (params (OtherActor :type "Actor Object Reference"))
  (bind _faction (`/Game/Enterotest/PropheteBp.Faction` (`self.Monprophete`)))
  (bind (_nom _color) (break `/Game/Faction` _faction))
  (if (!= (`self.Monprophete`) null)
    (bind _asfidele (cast `/Game/Fidele` OtherActor))
    (bind _nom_2 (break `/Game/Faction` (`/Game/Fidele.Faction` _asfidele)))
    (if (`KismetStringLibrary.EqualEqual_StrStr` _nom_2 _nom)
      _
      (elif (`KismetStringLibrary.EqualEqual_StrStr` _nom_2 "Neutre")
        (bind _staticmesh (`/Game/Fidele.StaticMesh` _asfidele))
        (bind _returnvalue (`PrimitiveComponent.CreateDynamicMaterialInstance` _staticmesh 0 (`PrimitiveComponent.GetMaterial` _staticmesh 0)))
        (`MaterialInstanceDynamic.SetVectorParameterValue` _returnvalue "Main Color" _color)
        (set `/Game/Fidele.Faction` _faction _asfidele)))))

(event `self.ReceiveBeginPlay`)

(event `self.ReceiveTick`
  (params (DeltaSeconds :type "Float (single-precision)"))
  (bind _returnvalue (`self.K2_GetActorLocation` (`self.Monprophete`)))
  (bind _overlappingactors (`PrimitiveComponent.GetOverlappingActors` (`self.Sphere`) "/Game/Fidele.Fidele_C"))
  (bind _worldlocation (`PlayerController.DeprojectMousePositionToWorld` (`GameplayStatics.GetPlayerController` 0)))
  (bind _nom (break `/Game/Faction` (`/Game/Enterotest/PropheteBp.Faction` (`self.Monprophete`))))
  (bind _returnvalue_2 (`self.K2_GetActorLocation` (`/Game/Enterotest/PropheteBp.Camera` (`self.Monprophete`))))
  (`self.K2_SetActorLocation` _returnvalue)
  (for _array_element _overlappingactors
    (bind _asfidele (cast `/Game/Fidele` _array_element))
    (if (`KismetStringLibrary.EqualEqual_StrStr` (`.Nom_3_A4A0DAA5406D709BC592F2906138E77E` (break `/Game/Faction` (`/Game/Fidele.Faction` _asfidele))) _nom)
      (if (`/Game/Enterotest/PropheteBp.InstructionGoAway` (`self.Monprophete`))
        (for _array_element_2 _overlappingactors
          (bind _asfidele_2 (cast `/Game/Fidele` _array_element_2))
          (set `/Game/Fidele.Destination` (`.Intersection` (`KismetMathLibrary.LinePlaneIntersection_OriginNormal` _returnvalue_2 (+ (* (- _worldlocation _returnvalue_2) 10000.0) _worldlocation) (0.0 0.0 0.0) (0.0 0.0 1.0))) _asfidele_2))
        (elif (`/Game/Enterotest/PropheteBp.InstructionFollowMe` (`self.Monprophete`))
          (for _array_element_3 _overlappingactors
            (bind _asfidele_3 (cast `/Game/Fidele` _array_element_3))
            (set `/Game/Fidele.Destination` _returnvalue _asfidele_3))
          (else
            (for _array_element_4 _overlappingactors
              (bind _asfidele_4 (cast `/Game/Fidele` _array_element_4))
              (set `/Game/Fidele.Destination` (-1.0 -1.0 -1.0) _asfidele_4)))))
      (elif (not (`KismetStringLibrary.EqualEqual_StrStr` _nom "Neutre"))
        (for _array_element_5 _overlappingactors
          (bind _asfidele_5 (cast `/Game/Fidele` _array_element_5))
          (set `/Game/Fidele.Destination` _returnvalue _asfidele_5))))))

(event `self.ReceiveActorBeginOverlap`
  (params (OtherActor :type "Actor Object Reference")))

(fn `UserConstructionScript`)